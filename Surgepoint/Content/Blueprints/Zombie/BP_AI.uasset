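; Zombie AI pawn that chases and melee-attacks the player and shows a damage popup when hit.
; AI perception toggles between a chase that re-issues its move every two seconds and plays an attack montage on arrival, and a patrol around the sensed stimulus location.
; Patrol picks random reachable points in a radius that doubles after each successful move and resets on chase.
; Health reduction and death logic is disconnected and never runs.
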(event OnTargetPerceptionUpdated(AIPerception)
  (params (Actor :type Actor%20Object%20Reference) (Stimulus :type AI%20Stimulus%20Structure))
  (if (.bsuccessfullysensed Stimulus)
    (Variables|Default|SetbCanSeePlayer? true)
    (CallFunction|ChasePlayer)
    (else
      (Variables|Default|SetbCanSeePlayer? false)
      (CallFunction|Patrol (.stimuluslocation Stimulus)))))

(event Custom|ChasePlayer
  (if (Variables|Default|GetbCanSeePlayer?)
    (Variables|Default|SetRadiusOrigin 3e+02)
    (AI|AIMoveTo self "0, 0, 0" (Game|GetPlayerCharacter 0) 1e+02 false
      (:then
        (Utilities|FlowControl|Delay 2.0)
        (CallFunction|ChasePlayer))
      (:OnSuccess
        (CallFunction|AttackPlayer)))))

(event Custom|Patrol
  (params (Origin :type Vector%20%28by%20ref%29))
  (if (Variables|Default|GetbCanSeePlayer?)
    (CallFunction|ChasePlayer)
    (else
      (AI|AIMoveTo self (.RandomLocation (AI|Navigation|GetRandomReachablePointinRadius Origin (Variables|Default|GetRadiusOrigin) 0 0)) 0 1e+02 false
        (:OnSuccess
          (Utilities|FlowControl|Delay 2.0)
          (Variables|Default|SetRadiusOrigin (* (Variables|Default|GetRadiusOrigin) 2.0))
          (CallFunction|Patrol Origin))))))

(event Custom|AttackPlayer
  (Animation|Montage|PlayMontage (Variables|Character|GetMesh) "/Game/Externals/BSP_ZombieAnims/Animations/Standing/Attack/Zombie_Attack_Standing.Zombie_Attack_Standing"
    (:OnCompleted
      (CallFunction|ChasePlayer))))

(event Game|Damage|EventPointDamage
  (params (Damage :type Float%20%28single-precision%29) (DamageType :type Damage%20Type%20Object%20Reference) (HitLocation :type Vector :default "0, 0, 0") (HitNormal :type Vector :default "0, 0, 0") (HitComponent :type Primitive%20Component%20Object%20Reference) (BoneName :type Name :default "None") (ShotFromDirection :type Vector :default "0, 0, 0") (InstigatedBy :type Controller%20Object%20Reference) (DamageCauser :type Actor%20Object%20Reference) (HitInfo :type Hit%20Result%20Structure%20%28by%20ref%29))
  (Game|SpawnActorfromClass "/Game/Externals/Demo_CrosshairSystem/ThirdPerson/BP_DamagePopUp.BP_DamagePopUp_C" (Math|Conversions|ToTransform(Vector) HitLocation) "Undefined" "MultiplyWithRoot" 0 Damage 0))

(fn ConstructionScript)