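; A construction-script Blueprint that builds a string of lanterns hanging along an editable spline wire.
; It adds a spline mesh per spline segment to form the wire, with adjustable thickness.
; It then spaces the requested number of static meshes evenly by spline distance, leaving both ends empty and optionally rotating them to follow the spline.
; LanternScale overrides the initial flag-size scale on each mesh, and no runtime logic exists.
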(event EventBeginPlay)

(event Collision|EventActorBeginOverlap
  (params (OtherActor :type Actor%20Object%20Reference)))

(event EventTick
  (params (DeltaSeconds :type Float%20%28single-precision%29)))

(fn ConstructionScript
  (bind _spline1 (Variables|Default|GetSpline1))
  (bind _thickness_of_the_wire (Variables|Default|GetThickness%20of%20the%20wire))
  (bind _number_of_meshes (Variables|Default|GetNumber%20of%20meshes))
  (bind _returnvalue (+ _number_of_meshes 2))
  (bind _returnvalue_2 (- _returnvalue 1))
  (Utilities|FlowControl|Sequence
    (:then_0
      ;[1 1 1] Generate Wire
      (for _index (range 0 (- (Spline|GetNumberOfSplinePoints (Variables|Default|GetSpline1)) 2))
        (bind _returnvalue_3 (AddComponent|AddSplineMeshComponent true (Math|Transform|MakeTransform "0, 0, 0" "0, 0, 0" (Math|Vector|MakeVector (Variables|Default|GetWire_Length) _thickness_of_the_wire _thickness_of_the_wire))))
        (Class|SceneComponent|Attachto _returnvalue_3 (Variables|Default|GetMAIN) "None" "KeepRelativeOffset" true)
        (SplineMesh|SetStartandEnd _returnvalue_3 (.Location (Spline|GetLocationandTangentatSplinePoint _spline1 _index "Local")) (.Tangent (Spline|GetLocationandTangentatSplinePoint _spline1 _index "Local")) (.Location (Spline|GetLocationandTangentatSplinePoint _spline1 (+ _index 1) "Local")) (.Tangent (Spline|GetLocationandTangentatSplinePoint _spline1 (+ _index 1) "Local")) true :!class /Script/Engine.SplineMeshComponent)))
    (:then_1
      (if (> _returnvalue 0)
        (for _index_2 (range 1 _returnvalue_2) ; Repeat loop for each mesh to add
          (if (not (== _index_2 _returnvalue_2))
            (bind _returnvalue_4 (AddComponent|AddStaticMeshComponent false (Math|Transform|MakeTransform (Math|Transform|InverseTransformLocation (Transformation|GetActorTransform) (Spline|GetLocationatDistanceAlongSpline (Variables|Default|GetSpline1) (* _index_2 (/ (Spline|GetSplineLength (Variables|Default|GetSpline1)) (Math|Conversions|ToFloat(Integer) _returnvalue_2))) "World")) "0, 0, 0" (* (Variables|Default|GetMesh_Size_Vector) (Variables|Default|GetSize%20of%20each%20flag))))) ; Add static mesh component
            (Transformation|SetRelativeScale3D _returnvalue_4 (Variables|Default|GetLanternScale))
            (if (Variables|Default|GetOrient%20to%20spline)
              (Transformation|SetWorldRotation _returnvalue_4 (Spline|GetRotationatDistanceAlongSpline (Variables|Default|GetSpline1) (* _index_2 (/ (Spline|GetSplineLength (Variables|Default|GetSpline1)) (Math|Conversions|ToFloat(Integer) _returnvalue_2))) "World") false false) ; Rotate mesh to match direction of spline at its position
            )))))))