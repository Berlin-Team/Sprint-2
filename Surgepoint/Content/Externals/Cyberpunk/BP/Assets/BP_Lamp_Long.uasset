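; Two-sided cyberpunk street lamp prop with holographic planes, point and spot lights, god rays and lens flares, configured entirely in the construction script.
; Each plane gets a dynamic material with random glow color, selection, scroll speed and gradient power.
; Point lights share exposed intensity and color.
; Flags destroy either side, all lights or single point lights; side removal and kill also swap the lamp mesh to its off material.
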(event EventBeginPlay)

(event Collision|EventActorBeginOverlap
  (params (OtherActor :type Actor%20Object%20Reference)))

(event EventTick
  (params (DeltaSeconds :type Float%20%28single-precision%29)))

(fn ConstructionScript
  (bind _plane2 (Variables|Components|GetPlane2))
  (bind _plane (Variables|Components|GetPlane))
  (bind _lamp_street (Variables|Components|GetLamp_Street))
  (bind _pointlight (Variables|Components|GetPointLight))
  (bind _point_intensity (Variables|Default|GetPoint%20Intensity))
  (bind _pointlight1 (Variables|Components|GetPointLight1))
  (bind _point_color (Variables|Default|GetPoint%20COlor))
  (Utilities|FlowControl|Sequence
    (:then_0
      (bind _returnvalue (Rendering|Material|CreateDynamicMaterialInstance (Rendering|Material|GetMaterial _plane 0) "None" "None" :!class /Script/Engine.KismetMaterialLibrary))
      (Rendering|Material|SetVectorParameterValue _returnvalue "Glow COlor" (Utilities|Array|Get(acopy) (Variables|Default|GetHolo%20COlor) (Math|Random|RandomIntegerinRange 0 3)) :!class /Script/Engine.MaterialInstanceDynamic)
      (Rendering|Material|SetScalarParameterValue _returnvalue "Select" (Math|Random|RandomFloatinRange 0.0 1.0) :!class /Script/Engine.MaterialInstanceDynamic)
      (Rendering|Material|SetScalarParameterValue _returnvalue "Speed" (Math|Random|RandomFloatinRange -0.15 -0.05) :!class /Script/Engine.MaterialInstanceDynamic)
      (Rendering|Material|SetScalarParameterValue _returnvalue "Gradien Power" (Math|Random|RandomFloatinRange 3.0 5.0) :!class /Script/Engine.MaterialInstanceDynamic)
      (Rendering|Material|SetMaterial _plane 0 _returnvalue))
    (:then_1
      (bind _returnvalue_2 (Rendering|Material|CreateDynamicMaterialInstance (Rendering|Material|GetMaterial _plane2 0) "None" "None" :!class /Script/Engine.KismetMaterialLibrary))
      (Rendering|Material|SetVectorParameterValue _returnvalue_2 "Glow COlor" (Utilities|Array|Get(acopy) (Variables|Default|GetHolo%20COlor) (Math|Random|RandomIntegerinRange 0 3)) :!class /Script/Engine.MaterialInstanceDynamic)
      (Rendering|Material|SetScalarParameterValue _returnvalue_2 "Select" (Math|Random|RandomFloatinRange 0.0 1.0) :!class /Script/Engine.MaterialInstanceDynamic)
      (Rendering|Material|SetScalarParameterValue _returnvalue_2 "Speed" (Math|Random|RandomFloatinRange -0.15 -0.05) :!class /Script/Engine.MaterialInstanceDynamic)
      (Rendering|Material|SetScalarParameterValue _returnvalue_2 "Gradien Power" (Math|Random|RandomFloatinRange 3.0 5.0) :!class /Script/Engine.MaterialInstanceDynamic)
      (Rendering|Material|SetMaterial _plane2 0 _returnvalue_2))
    (:then_2
      (Rendering|Components|Light|SetIntensity _pointlight _point_intensity)
      (Rendering|Components|Light|SetLightColor _pointlight _point_color true)
      (Rendering|Components|Light|SetIntensity _pointlight1 _point_intensity)
      (Rendering|Components|Light|SetLightColor _pointlight1 _point_color true))
    (:then_6
      (if (Variables|Default|GetRemove%20Left)
        (Components|DestroyComponent (Variables|Components|GetPointLight))
        (Rendering|Material|SetMaterial _lamp_street 0 "/Game/Externals/Cyberpunk/Materials/Instances/MI_LampSTreet_Off.MI_LampSTreet_Off" :!label _label)
        (Rendering|Material|SetMaterial _lamp_street 1 "/Game/Externals/Cyberpunk/Materials/Instances/MI_LampSTreet_Off.MI_LampSTreet_Off")))
    (:then_7
      (if (Variables|Default|GetRemove%20Right)
        (Components|DestroyComponent (Variables|Components|GetSpotLight1))
        (goto _label)))
    (:then_8
      ;[1 1 1] Kill Lights
      (if (Variables|Default|GetKill%20Light)
        (Components|DestroyComponent (Variables|Components|GetPointLight1))
        (goto _label)))
    (:then_9
      (if (Variables|Default|GetDisable%20Point%20LT)
        (bind _pointlight1_2 (Variables|Components|GetPointLight1)
          (:then
            (Components|DestroyComponent _pointlight1_2))
          (:else))))
    (:then_10
      (if (Variables|Default|GetDisable%20Point%20RT)
        (bind _pointlight_2 (Variables|Components|GetPointLight)
          (:then
            (Components|DestroyComponent _pointlight_2))
          (:else))))))