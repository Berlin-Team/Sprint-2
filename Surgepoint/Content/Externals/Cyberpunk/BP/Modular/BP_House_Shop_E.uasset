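; Modular cyberpunk shop building whose floors, foundation trim, roof, billboards and lights are configured per instance in the Construction Script.
; Boolean flags destroy the components of unwanted sections and set negative height offsets, which are summed to lower the remaining upper floors and roof.
; Type indices pick first-floor, roof and balcony meshes from arrays.
; The event graph is empty, and the emissive material assignments are disconnected.
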(event EventBeginPlay)

(event Collision|EventActorBeginOverlap
  (params (OtherActor :type Actor%20Object%20Reference)))

(event EventTick
  (params (DeltaSeconds :type Float%20%28single-precision%29)))

(fn ConstructionScript
  (bind _floor_1_type (Variables|Default|GetFloor%201%20Type))
  (bind _balcon_array (Variables|Default|GetBalcon%20Array))
  (Utilities|FlowControl|Sequence
    (:then_0
      ;[1 1 1] Floor 4
      (if (Variables|Default|GetFloor%204)
        (Components|DestroyComponent (Variables|Default|GetHouse_Shop_H_Front))
        (LocalVariables|SetFloor%204%20Offset -4.5e+02)))
    (:then_1
      ;[1 1 1] Floor 3
      (if (Variables|Default|GetFloor%203)
        (Components|DestroyComponent (Variables|Default|GetHouse_Shop_G_Front))
        (LocalVariables|SetFloor%203%20Offset -4.5e+02)))
    (:then_2
      ;[1 1 1] Floor  2
      (if (Variables|Default|GetFloor%202)
        (Components|DestroyComponent (Variables|Default|GetHouse_Shop_F_Front))
        (Components|DestroyComponent (Variables|Default|GetRoof_Corner_Out))
        (Components|DestroyComponent (Variables|Default|GetBeam_Border_Corner11))
        (Components|DestroyComponent (Variables|Default|GetBeam_Concrete_02))
        (LocalVariables|SetFloor%202%20Offset -5e+02)))
    (:then_3
      ;[1 1 1] Floor 1
      (if (Variables|Default|GetFloor%201)
        (Components|DestroyComponent (Variables|Default|GetHouse_Shop_E_Front))
        (Components|DestroyComponent (Variables|Default|GetRoof_Small_Corner2))
        (Components|DestroyComponent (Variables|Default|GetBeam_Border_Corner4))
        (Components|DestroyComponent (Variables|Default|GetHouse_Shop_E_Corner7))
        (LocalVariables|SetFloor%201%20Offset -5e+02)
        (else
          (Components|StaticMesh|SetStaticMesh (Variables|Default|GetHouse_Shop_E_Front) (Utilities|Array|Get(acopy) (Variables|Default|GetFloor%201%20Array) _floor_1_type))
          (Utilities|FlowControl|Sequence
            (:then_0
              (if (!= _floor_1_type 1)
                (Components|DestroyComponent (Variables|Default|GetPointLight8))))))))
    (:then_4
      ;[1 1 1] Fundament
      (if (Variables|Default|GetFundament)
        (Components|DestroyComponent (Variables|Default|GetBorder_House_600))))
    (:then_5
      ;[1 1 1] Comment
      (if (and (Variables|Default|GetFloor%204) (Variables|Default|GetFloor%203))
        (Components|DestroyComponent (Variables|Default|GetRoof_Corner_Out))
        (Components|DestroyComponent (Variables|Default|GetBeam_Border_Corner11))
        (LocalVariables|SetRoof%20Offset -1e+02)))
    (:then_6
      ;[1 1 1] Roof
      (Utilities|FlowControl|Sequence
        (:then_0
          (if (Variables|Default|GetRoof%20Top)
            (Components|DestroyComponent (Variables|Default|GetRoof_Square))
            (Components|DestroyComponent (Variables|Default|GetBeam_Border_Corner8))
            (Components|DestroyComponent (Variables|Default|GetBeam_Concrete_08))
            (else
              (Components|StaticMesh|SetStaticMesh (Variables|Default|GetRoof_Square) (Utilities|Array|Get(acopy) (Variables|Default|GetRoof%20Array) (Variables|Default|GetRoof%20Type))))))))
    (:then_7
      ;[1 1 1] Offset floor
      (Utilities|FlowControl|Sequence
        (:then_0
          (bind _roof_square (Variables|Default|GetRoof_Square)
            (:then
              (Transformation|AddRelativeLocation _roof_square (Math|Vector|MakeVector 0.0 0.0 (+ (LocalVariables|GetFloor%202%20Offset) (LocalVariables|GetFloor%203%20Offset) (LocalVariables|GetFloor%204%20Offset) (LocalVariables|GetRoof%20Offset) (LocalVariables|GetFloor%201%20Offset))) false false))
            (:else)))
        (:then_1
          (bind _house_shop_h_front (Variables|Default|GetHouse_Shop_H_Front)
            (:then
              (Transformation|AddRelativeLocation _house_shop_h_front (Math|Vector|MakeVector 0.0 0.0 (+ (LocalVariables|GetFloor%203%20Offset) (LocalVariables|GetFloor%202%20Offset) (LocalVariables|GetFloor%201%20Offset))) false false))
            (:else)))
        (:then_2
          (bind _house_shop_f_front (Variables|Default|GetHouse_Shop_F_Front)
            (:then
              (Transformation|AddRelativeLocation _house_shop_f_front (Math|Vector|MakeVector 0.0 0.0 (LocalVariables|GetFloor%201%20Offset)) false false))
            (:else)))
        (:then_3
          (bind _house_shop_g_front (Variables|Default|GetHouse_Shop_G_Front)
            (:then
              (Transformation|AddRelativeLocation _house_shop_g_front (Math|Vector|MakeVector 0.0 0.0 (+ (LocalVariables|GetFloor%201%20Offset) (LocalVariables|GetFloor%202%20Offset))) false false))
            (:else)))))
    (:then_8
      ;[1 1 1] Comment
      (Utilities|FlowControl|Sequence
        (:then_0
          (bind _balkon_grid_01 (Variables|Default|GetBalkon_Grid_01)
            (:then
              (Components|StaticMesh|SetStaticMesh _balkon_grid_01 (Utilities|Array|Get(acopy) _balcon_array (Variables|Default|GetBalkon%20A%20Type))))
            (:else)))
        (:then_1
          (bind _balkon_grid_02 (Variables|Default|GetBalkon_Grid_02)
            (:then
              (Components|StaticMesh|SetStaticMesh _balkon_grid_02 (Utilities|Array|Get(acopy) _balcon_array (Variables|Default|GetBalkon%20B%20Type))))
            (:else)))))
    (:then_9
      ;[1 1 1] Billboard
      (Utilities|FlowControl|Sequence
        (:then_0
          (if (Variables|Default|GetRemove%20Billboard%20Long)
            (Components|DestroyComponent (Variables|Default|GetBillboard_SIde_Long_03))))
        (:then_1
          (if (Variables|Default|GetRemove%20Billboard%20Short)
            (Components|DestroyComponent (Variables|Default|GetBillboard_SIde_Square))))))
    (:then_10
      (if (Variables|Default|GetKill%20ALl%20Lights)
        (for _array_element (Utilities|Array|MakeArray (Variables|Default|GetPointLight1) (Variables|Default|GetPointLight9) (Variables|Default|GetPointLight10) (Variables|Default|GetPointLight11) (Variables|Default|GetPointLight) (Variables|Default|GetPointLight7) (Variables|Default|GetPointLight8) (Variables|Default|GetPointLight6) (Variables|Default|GetPointLight3) (Variables|Default|GetPointLight4) (Variables|Default|GetPointLight5) (Variables|Default|GetPointLight2))
          (Utilities|IsValid _array_element
            (:Is%20Valid
              (Components|DestroyComponent _array_element))))))))