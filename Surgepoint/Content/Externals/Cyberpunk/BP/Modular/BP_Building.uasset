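; Modular three-floor building actor, configured entirely in the construction script with no active runtime logic.
; Each floor's wall type picks a mesh from WallArray and decides which prebuilt windows, extra wall/floor/column pieces and point lights survive.
; Boolean options strip left or right columns, side handrails, side walls or all lights.
; Variants work by destroying unneeded components rather than spawning them; emissive material assignment is present but disconnected.
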(event EventBeginPlay)

(event Collision|EventActorBeginOverlap
  (params (OtherActor :type Actor%20Object%20Reference)))

(event EventTick
  (params (DeltaSeconds :type Float%20%28single-precision%29)))

(fn ConstructionScript
  (bind _wall_array (Variables|Default|GetWall_Array))
  (bind _wall_type_floor_1 (Variables|Default|GetWall%20Type%20Floor%201))
  (bind _wall_type_floor_2 (Variables|Default|GetWall%20Type%20Floor%202))
  (bind _wall_type_floor_3 (Variables|Default|GetWall%20Type%20Floor%203))
  (Utilities|FlowControl|Sequence
    (:then_0
      ;[1 1 1] Column Left
      (if (Variables|Default|GetRemove%20Column%20Left)
        (Components|DestroyComponent (Variables|Default|GetBuilding_Column_C))
        (Components|DestroyComponent (Variables|Default|GetBuilding_Column_A3))))
    (:then_1
      ;[1 1 1] Comment
      (if (Variables|Default|GetRemove%20Column%20Right)
        (Components|DestroyComponent (Variables|Default|GetBuilding_Column_A8))))
    (:then_2
      ;[1 1 1] Comment
      (if (Variables|Default|GetRemove%20Handrails%20Side)
        (Components|DestroyComponent (Variables|Default|GetBalcon_Wood_Handrail6))
        (Components|DestroyComponent (Variables|Default|GetBalcon_Wood_Handrail14))))
    (:then_3
      ;[1 1 1] Comment
      (Utilities|FlowControl|Sequence
        (:then_0
          (Components|StaticMesh|SetStaticMesh (Variables|Default|GetBuilding_Wall_A) (Utilities|Array|Get(acopy) _wall_array _wall_type_floor_1))
          (if (!= _wall_type_floor_3 1)
            (Components|DestroyComponent (Variables|Default|GetWindow_C_V04))
            (Components|DestroyComponent (Variables|Default|GetPointLight1))))
        (:then_1
          (Components|StaticMesh|SetStaticMesh (Variables|Default|GetBuilding_Wall_A1) (Utilities|Array|Get(acopy) _wall_array _wall_type_floor_2))
          (if (!= _wall_type_floor_2 1)
            (Components|DestroyComponent (Variables|Default|GetWindow_C_V010))
            (Components|DestroyComponent (Variables|Default|GetPointLight4))))
        (:then_2
          (Components|StaticMesh|SetStaticMesh (Variables|Default|GetBuilding_Wall_A2) (Utilities|Array|Get(acopy) _wall_array _wall_type_floor_3))
          (if (!= _wall_type_floor_1 1)
            (Components|DestroyComponent (Variables|Default|GetWindow_C_V016))
            (Components|DestroyComponent (Variables|Default|GetPointLight6))))
        (:then_3
          (Utilities|FlowControl|Sequence
            (:then_0
              (if (!= _wall_type_floor_1 3)
                (Components|DestroyComponent (Variables|Default|GetBuilding_Floor_A3))
                (Components|DestroyComponent (Variables|Default|GetPointLight14))))
            (:then_1
              (if (!= _wall_type_floor_2 3)
                (Components|DestroyComponent (Variables|Default|GetBuilding_Floor_A6))
                (Components|DestroyComponent (Variables|Default|GetPointLight11))))
            (:then_2
              (if (!= _wall_type_floor_3 3)
                (Components|DestroyComponent (Variables|Default|GetBuilding_Floor_A10))
                (Components|DestroyComponent (Variables|Default|GetPointLight9))))))
        (:then_4
          (Utilities|FlowControl|Sequence
            (:then_0
              (if (!= _wall_type_floor_1 2)
                (Components|DestroyComponent (Variables|Default|GetPointLight8))))
            (:then_1
              (if (!= _wall_type_floor_2 2)
                (Components|DestroyComponent (Variables|Default|GetPointLight5))))
            (:then_2
              (if (!= _wall_type_floor_3 2)
                (Components|DestroyComponent (Variables|Default|GetPointLight2))))))))
    (:then_4
      ;[1 1 1] Side walls
      (if (Variables|Default|GetRemove%20Side%20Walls)
        (Components|DestroyComponent (Variables|Default|GetBuilding_Wall_A7))))
    (:then_5
      ;[1 1 1] Kill lights
      (if (Variables|Default|GetRemove%20All%20Lights)
        (for _array_element (Utilities|Array|MakeArray (Variables|Default|GetPointLight7) (Variables|Default|GetPointLight1) (Variables|Default|GetPointLight2) (Variables|Default|GetPointLight3) (Variables|Default|GetPointLight) (Variables|Default|GetPointLight5) (Variables|Default|GetPointLight6) (Variables|Default|GetPointLight4) (Variables|Default|GetPointLight8) (Variables|Default|GetPointLight9) (Variables|Default|GetPointLight10) (Variables|Default|GetPointLight11) (Variables|Default|GetPointLight12) (Variables|Default|GetPointLight13) (Variables|Default|GetPointLight14))
          (Utilities|IsValid _array_element
            (:Is%20Valid
              (Components|DestroyComponent _array_element))))))))